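; BP_Enemy is an enemy that turns to face the player and plays attack animations at close range.
; While the player is inside DetectSphere, Tick rotates only the mesh's yaw toward them, offset by 90 degrees.
; Overlapping AttackDetect plays the LightAttack montage, which replays on completion through the Attack event until the player leaves that volume.
; It contains no movement or damage logic.
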(event `self.ReceiveTick`
  (params (DeltaSeconds :type "Float (single-precision)"))
  (bind (_returnvalue_roll _returnvalue_pitch _returnvalue_yaw) (`KismetMathLibrary.BreakRotator` (`KismetMathLibrary.FindLookAtRotation` (`self.K2_GetActorLocation`) (`self.K2_GetActorLocation` (`GameplayStatics.GetPlayerCharacter` 0)))))
  ;[1 0.09154 0] Look at me
  (if (`self.ZoneDetect`)
    (`SceneComponent.K2_SetWorldRotation` (`self.Mesh`) (`KismetMathLibrary.MakeRotator` 0.0 0.0 (- _returnvalue_yaw 90.0)) false false)))

(event `self.DetectSphere.OnComponentBeginOverlap`
  (params (OverlappedComponent :type "PrimitiveComponent Object Reference") (OtherActor :type "Actor Object Reference") (OtherComp :type "PrimitiveComponent Object Reference") (OtherBodyIndex :type Integer) (bFromSweep :type Boolean) (SweepResult :type "HitResult Structure (by ref)"))
  ;[0 0.2052 1] Zone detect
  (if (== OtherActor (`GameplayStatics.GetPlayerCharacter` 0))
    (set `self.ZoneDetect` true)))

(event `self.DetectSphere.OnComponentEndOverlap`
  (params (OverlappedComponent :type "PrimitiveComponent Object Reference") (OtherActor :type "Actor Object Reference") (OtherComp :type "PrimitiveComponent Object Reference") (OtherBodyIndex :type Integer))
  ;[0 0.2052 1] Zone detect
  (if (== (`GameplayStatics.GetPlayerCharacter` 0) OtherActor)
    (set `self.ZoneDetect` false)))

(event `self.AttackDetect.OnComponentBeginOverlap`
  (params (OverlappedComponent :type "PrimitiveComponent Object Reference") (OtherActor :type "Actor Object Reference") (OtherComp :type "PrimitiveComponent Object Reference") (OtherBodyIndex :type Integer) (bFromSweep :type Boolean) (SweepResult :type "HitResult Structure (by ref)"))
  ;[1 0 0.006631] Attack detect
  (if (== OtherActor (`GameplayStatics.GetPlayerCharacter` 0))
    (set `self.Attack` true)
    (`|PlayMontage` (`self.Mesh`) "/Game/Sword_Animations/Animations/Sequence1/02_Attack/03_Combo_Attack_03/LightAttack.LightAttack" :!label _label
      (:`OnCompleted`
        (if (`self.Attack`)
          (`self.Attack `))))))

(event `Attack`
  ;[1 0 0.006631] Attack detect
  (goto _label))

(event `self.AttackDetect.OnComponentEndOverlap`
  (params (OverlappedComponent :type "PrimitiveComponent Object Reference") (OtherActor :type "Actor Object Reference") (OtherComp :type "PrimitiveComponent Object Reference") (OtherBodyIndex :type Integer))
  ;[1 0 0.006631] Attack detect
  (if (== (`GameplayStatics.GetPlayerCharacter` 0) OtherActor)
    (set `self.Attack` false)))

(fn `UserConstructionScript`)